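; Audio equalizer controller that turns a grid of spawned cubes into a spectrum visualizer.
; On BeginPlay it opens test media at reduced volume, spawns a square-rooted row layout of Cube_BP actors and optionally shuffles them to scatter the bands.
; Each Tick computes the frequency spectrum of AudioTrack at current game time, one band per cube, and drives each cube's Z scale.
; The analyzed SoundWave is set separately from the played media.
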(event EventBeginPlay
  (Audio|Components|Audio|SetVolumeMultiplier (Variables|Default|GetMediaSound) 0.4 :!class /Script/AudioMixer.SynthComponent)
  (Media|MediaPlayer|OpenSource (Variables|Default|GetmediaPlayer) "/Game/Media/testMedia.testMedia")
  (CallFunction|SpawnGrid)
  (if (Variables|Default|Getshuffle)
    (Utilities|Array|Shuffle (Variables|Default|GetcubeArray))))

(event EventTick
  (params (DeltaSeconds :type Float%20%28single-precision%29))
  (bind _outspectrum (Class|SoundVisualizationStatics|CalculateFrequencySpectrum (Variables|Default|GetaudioTrack) 0 (Utilities|Time|GetGameTimeinSeconds) 0.1 (Utilities|Array|Length (Variables|Default|GetcubeArray))))
  (Variables|Default|Setspectrum _outspectrum)
  (for (_array_element _array_index) (Variables|Default|GetcubeArray)
    (Transformation|SetActorScale3D _array_element (Math|Vector|MakeVector 1.0 1.0 (* (Math|Float|Absolute(Float) (Utilities|Array|Get(acopy) (Variables|Default|Getspectrum) _array_index)) 0.2)))))

(fn ConstructionScript)

(fn SpawnGrid
  (bind _distance (Variables|Default|Getdistance))
  (for _index (range 0 (- (Variables|Default|GetnumCubes) 1))
    (bind _returnvalue (Game|SpawnActorfromClass "/Game/Blueprint/cube_BP.cube_BP_C" (Math|Transform|MakeTransform (Math|Vector|MakeVector (* (Variables|Default|GetRow) _distance) (* (Variables|Default|GetCol) _distance) 0.0) "0, 0, 0" "1,1,1") "AlwaysSpawn" 0 0))
    (Utilities|Array|Add (Variables|Default|GetcubeArray) _returnvalue)
    (Math|Integer|IncrementInt (Variables|Default|GetRow)
      (:%20%20
        (if (== (Variables|Default|GetRow) (Math|Float|Truncate (Math|Float|Sqrt (Math|Conversions|ToFloat(Integer) (Variables|Default|GetnumCubes)))))
          (Math|Integer|IncrementInt (Variables|Default|GetCol)
            (:%20%20
              (Variables|Default|SetRow 0))))))))